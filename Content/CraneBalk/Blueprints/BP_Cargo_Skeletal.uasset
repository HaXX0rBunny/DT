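; Skeletal-mesh cargo actor that a crane can attach and detach, extending a parent cargo class with optional looping animation.
; Attaching disables physics; detaching without carried physics immediately snaps the actor location and BoundBox rotation to the mesh.
; Enabling physics unpauses a looping timer that polls until all bodies sleep, then pauses and performs the same realignment.
; Spot and Unspot toggle custom depth rendering, while SetCargoMesh assigns the mesh and returns its location and bounds.
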(event Custom|CheckBodySimulation
  ;[1 1 1] Check that any rigid body already no physic simulation
  (if (not (Class|PrimitiveComponent|IsAnyRigidBodyAwake (Variables|Default|GetSkeletalMesh)))
    (Utilities|Time|PauseTimerbyHandle (Variables|Default|GetCheckRigidBodyHandle))
    (CallFunction|InitCargoActor)))

(event Custom|InitCargoActor
  (bind _skeletalmesh (Variables|Default|GetSkeletalMesh))
  (bind _returnvalue (Transformation|GetWorldTransform _skeletalmesh))
  ;[1 1 1] Detach
  (Transformation|SetActorLocation (.location _returnvalue) false true)
  (Transformation|SetWorldRotation (Variables|Default|GetBoundBox) (.rotation _returnvalue) false false))

(event EventBeginPlay
  (bind _skeletalmesh (Variables|Default|GetSkeletalMesh))
  (bind _animtoplay (Variables|Cargo|GetAnimToPlay))
  ;[1 1 1] Init timer for check physic simulation
  (|CallParentFunction)
  (bind _returnvalue (Utilities|Time|SetTimerbyFunctionName self "CheckBodySimulation" 0.5 true))
  (bind _output_get (Variables|Default|SetCheckRigidBodyHandle _returnvalue))
  (Utilities|Time|PauseTimerbyHandle _output_get)
  (Utilities|IsValid _skeletalmesh
    (:Is%20Valid
      (Utilities|IsValid _animtoplay
        (:Is%20Valid
          (Components|Animation|PlayAnimation _skeletalmesh _animtoplay true))))))

(event Collision|EventActorBeginOverlap
  (params (OtherActor :type Actor%20Object%20Reference))
  (|CallParentFunction OtherActor) ; This node is disabled and will not be called.\nDrag off pins to build functionality.
)

(event EventTick
  (params (DeltaSeconds :type Float%20%28single-precision%29))
  (|CallParentFunction DeltaSeconds) ; This node is disabled and will not be called.\nDrag off pins to build functionality.
)

(event EventAttachtoCrane
  (params (Component :type Arrow%20Component%20Object%20Reference))
  (bind _skeletalmesh (Variables|Default|GetSkeletalMesh))
  ;[1 1 1] Attach
  (Physics|SetSimulatePhysics _skeletalmesh false)
  (Transformation|AttachComponentToComponent _skeletalmesh Component "None" "KeepWorld" "KeepWorld" "KeepWorld" true))

(event EventDetachfromCrane
  (bind _skeletalmesh (Variables|Default|GetSkeletalMesh))
  (bind _returnvalue (Transformation|GetWorldTransform _skeletalmesh))
  ;[1 1 1] Detach
  (Transformation|DetachFromComponent _skeletalmesh "KeepWorld" "KeepWorld" "KeepWorld" false)
  (if (not (Variables|Default|GetEnablePhysicWhenCarried))
    (Transformation|SetActorLocation (.location _returnvalue) false true)
    (Transformation|SetWorldRotation (Variables|Default|GetBoundBox) (.rotation _returnvalue) false false)))

(event EventEnableCargoPhysic
  ;[1 1 1] Enable Physic
  (Physics|SetSimulatePhysics (Variables|Default|GetSkeletalMesh) true)
  (Utilities|Time|UnpauseTimerbyHandle (Variables|Default|GetCheckRigidBodyHandle)))

(event EventSpot
  ;[1 1 1] Enable custom Depth render
  (Rendering|SetRenderCustomDepth (Variables|Default|GetSkeletalMesh) true))

(event EventUnspot
  ;[1 1 1] Disable suctom Depth render
  (Rendering|SetRenderCustomDepth (Variables|Default|GetSkeletalMesh) false))

(fn ConstructionScript
  (|CallParentFunction))

(fn SetCargoMesh
  (bind _skeletalmesh (Variables|Default|GetSkeletalMesh))
  ;[1 1 1] Set Skeletal mesh and return location and bounds
  (Variables|Default|SetCargoMeshComponent (Variables|Default|GetSkeletalMesh))
  (Class|SkinnedMeshComponent|SetSkeletalMesh _skeletalmesh (Variables|Cargo|GetCargo_SkeletalMesh) true)
  (return (Utilities|IsValid _skeletalmesh) (Transformation|GetWorldLocation _skeletalmesh) (.BoxExtent (Collision|GetComponentBounds _skeletalmesh))))