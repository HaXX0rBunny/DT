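; Crane cargo actor with a static mesh that can be attached, detached, switched to physics and highlighted through custom depth.
; Attaching turns off simulation, and detaching immediately resyncs the actor to the mesh unless EnablePhysicWhenCarried is set.
; Enabling physics unpauses a looping timer that waits for the body to sleep, then moves the actor and rotates BoundBox to match the mesh.
; SetCargoMesh applies the configured mesh and returns its location and bounds.
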(event Custom|CheckBodySimulation
  ;[1 1 1] Check that any rigid body already no physic simulation
  (if (not (Class|PrimitiveComponent|IsAnyRigidBodyAwake (Variables|Default|GetStaticMesh)))
    (Utilities|Time|PauseTimerbyHandle (Variables|Default|GetCheckRigidBodyHandle))
    (CallFunction|InitCargoActor)))

(event Custom|InitCargoActor
  (bind _staticmesh (Variables|Default|GetStaticMesh))
  (bind _returnvalue (Transformation|GetWorldTransform _staticmesh))
  ;[1 1 1] Detach
  (Transformation|SetActorLocation (.location _returnvalue) false true)
  (Transformation|SetWorldRotation (Variables|Default|GetBoundBox) (.rotation _returnvalue) false false))

(event EventBeginPlay
  ;[1 1 1] Init timer for check physic simulation
  (|CallParentFunction)
  (bind _returnvalue (Utilities|Time|SetTimerbyFunctionName self "CheckBodySimulation" 0.5 true))
  (bind _output_get (Variables|Default|SetCheckRigidBodyHandle _returnvalue))
  (Utilities|Time|PauseTimerbyHandle _output_get))

(event Collision|EventActorBeginOverlap
  (params (OtherActor :type Actor%20Object%20Reference))
  (|CallParentFunction OtherActor) ; This node is disabled and will not be called.\nDrag off pins to build functionality.
)

(event EventTick
  (params (DeltaSeconds :type Float%20%28single-precision%29))
  (|CallParentFunction DeltaSeconds) ; This node is disabled and will not be called.\nDrag off pins to build functionality.
)

(event EventAttachtoCrane
  (params (Component :type Arrow%20Component%20Object%20Reference))
  (bind _staticmesh (Variables|Default|GetStaticMesh))
  ;[1 1 1] Attach
  (Physics|SetSimulatePhysics _staticmesh false)
  (Transformation|AttachComponentToComponent _staticmesh Component "None" "KeepWorld" "KeepWorld" "KeepWorld" true))

(event EventDetachfromCrane
  (bind _staticmesh (Variables|Default|GetStaticMesh))
  (bind _returnvalue (Transformation|GetWorldTransform _staticmesh))
  ;[1 1 1] Detach
  (Transformation|DetachFromComponent _staticmesh "KeepWorld" "KeepWorld" "KeepWorld" false)
  (if (not (Variables|Default|GetEnablePhysicWhenCarried))
    (Transformation|SetActorLocation (.location _returnvalue) false true)
    (Transformation|SetWorldRotation (Variables|Default|GetBoundBox) (.rotation _returnvalue) false false)))

(event EventEnableCargoPhysic
  ;[1 1 1] Enable Physic
  (Physics|SetSimulatePhysics (Variables|Default|GetStaticMesh) true)
  (Utilities|Time|UnpauseTimerbyHandle (Variables|Default|GetCheckRigidBodyHandle)))

(event EventSpot
  ;[1 1 1] Enable custom Depth render
  (Rendering|SetRenderCustomDepth (Variables|Default|GetStaticMesh) true))

(event EventUnspot
  ;[1 1 1] Disable suctom Depth render
  (Rendering|SetRenderCustomDepth (Variables|Default|GetStaticMesh) false))

(fn ConstructionScript
  (|CallParentFunction))

(fn SetCargoMesh
  (bind _staticmesh (Variables|Default|GetStaticMesh))
  (bind _cargo_staticmesh (Variables|Cargo|GetCargo_StaticMesh))
  ;[1 1 1] Set Staic mesh and return location and bounds
  (Variables|Default|SetCargoMeshComponent _staticmesh)
  (bind _returnvalue (Components|StaticMesh|SetStaticMesh _staticmesh _cargo_staticmesh))
  (return _returnvalue (Transformation|GetWorldLocation _staticmesh) (.BoxExtent (Math|BoxSphereBounds|BreakBoxSphereBounds (StaticMesh|GetBounds _cargo_staticmesh)))))