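; BP_Cargo_Base is the overridable parent for crane cargo, with stub events for attach, detach, physics and custom-depth highlighting.
; Its construction script gets mesh location and bounds from a child-overridable SetCargoMesh, which fails by default, then fits BoundBox using optional auto bounds, offset and yaw.
; SpawnTarget creates a linked BP_Target that receives the bounds.
; It also tracks carried state and exposes the box transform, bounds and mesh component.
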(event Custom|AttachToCrane
  (params (Component :type Arrow%20Component%20Object%20Reference))
  ;[1 1 1] You can overwrite this events for making your own cargo type
  ;;[0 1 0.9057] Calling when need attach to Crane
)

(event Custom|DetachFromCrane
  ;[1 1 1] You can overwrite this events for making your own cargo type
  ;;[0 1 0.9057] Calling when need to detach from Crane
)

(event Custom|EnableCargoPhysic
  ;[1 1 1] You can overwrite this events for making your own cargo type
  ;;[0 1 0.9057] For Physic activation
)

(event Custom|Spot
  ;[1 1 1] You can overwrite this events for making your own cargo type
  ;;[0 1 0.9057] For Spot (enable Custom Depth render)
)

(event Custom|Unspot
  ;[1 1 1] You can overwrite this events for making your own cargo type
  ;;[0 1 0.9057] For Unspot (disable Custom Depth render)
)

(event Custom|SetCarried
  ;[1 1 1] You can overwrite this events for making your own cargo type
  ;;[0 1 0.9057] Mark Cargo is carried
  (Variables|Default|SetIsCarried true))

(event EventBeginPlay
  (Variables|Default|SetIsCarried false))

(event Collision|EventActorBeginOverlap
  (params (OtherActor :type Actor%20Object%20Reference)))

(event EventTick
  (params (DeltaSeconds :type Float%20%28single-precision%29)))

(fn ConstructionScript
  (bind _returnvalue (Transformation|GetActorRotation))
  (bind _target (Variables|Cargo|GetTarget))
  (bind _offset (Variables|Cargo|GetOffset))
  (bind _boundbox (Variables|Default|GetBoundBox))
  (bind _returnvalue_2 (Math|Vector|MakeVector (.x _offset) (.y _offset) 0.0))
  (bind _returnvalue_3 (Math|Vector|RotateVector _returnvalue_2 (Math|Rotator|MakeRotator 0.0 0.0 (.yaw _returnvalue))))
  (Transformation|SetActorScale3D "1.000000,1.000000,1.000000")
  (bind (_result _meshlocation _meshbounds) (Class|ICraneBalk|SetCargoMesh(Message) self))
  (if _result
    (Variables|Default|SetMeshLocation _meshlocation)
    (LocalVariables|SetTempBounds _meshbounds)
    (if (Variables|Cargo|GetAutoBounds)
      (Variables|Cargo|SetBounds (LocalVariables|GetTempBounds)))
    (Components|Box|SetBoxExtent _boundbox (Variables|Cargo|GetBounds) true)
    (Transformation|SetWorldLocation _boundbox (Variables|Default|GetMeshLocation) false false)
    (Transformation|AddWorldOffset (Variables|Default|GetBoundBox) (Math|Vector|MakeVector (.x _returnvalue_3) (.y _returnvalue_3) (.z _offset)) false false)
    (Transformation|SetWorldRotation (Variables|Default|GetBoundBox) (Math|Rotator|MakeRotator 0.0 0.0 (+ (Variables|Cargo|GetYawRotation) (.yaw _returnvalue))) false false)
    (Utilities|IsValid _target
      (:Is%20Valid
        (Default|UpdateBounds _target (Variables|Cargo|GetBounds))))))

(fn GetMeshLocationSize
  (return (Transformation|GetWorldLocation (Variables|Default|GetBoundBox)) (Variables|Cargo|GetBounds) (Transformation|GetWorldRotation (Variables|Default|GetBoundBox)) (.z (Variables|Cargo|GetOffset))))

(fn GetCargoMeshComp
  (return (Variables|Default|GetCargoMeshComponent)))

(fn SpawnTarget
  (bind _returnvalue (Game|SpawnActorfromClass "/Game/CraneBalk/Blueprints/BP_Target.BP_Target_C" (Math|Transform|MakeTransform (+ (.location (Transformation|GetActorTransform)) "250.000000, 0, 0") "0, 0, 0" "1,1,1") "Undefined" 0 0))
  (bind _output_get (Variables|Cargo|SetTarget _returnvalue))
  (Default|UpdateBounds _output_get (Variables|Cargo|GetBounds)))

(fn SetCargoMesh
  (return false "0, 0, 0" "0, 0, 0"))