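; BP_CargoSpawner creates a random cargo and a drop target for a manipulator robot, then starts the robot on it.
; SpawnCargo runs only in one robot state, otherwise reporting it busy.
; It places the cargo mesh and target independently in a random ring within the robot's reach, at random height offset by cargo bounds.
; It links target to cargo, calls InitCargoList on the robot, adds the cargo and calls Start.
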(event Custom|SpawnCargo
  (bind _manipulatorrobot (Variables|Default|GetManipulatorRobot))
  (bind _manipulatorrobot_2 (Variables|Default|GetManipulatorRobot))
  (bind _manipulatorrobot_3 (Variables|Default|GetManipulatorRobot))
  (if (Utilities|Enum|Equal(Enum) (Variables|/Game/ManipulatorRobot/Blueprints/ManipulatorRobot/ManipulatorRobot_BP.ManipulatorRobot_BP_C|Getstate (Variables|Default|GetManipulatorRobot)) "NewEnumerator0")
    (Development|PrintString "Spawn Cargo and Target")
    ;[1 1 1] Spawn random Cargo from the list at random location around the robot
    (bind _returnvalue (Game|SpawnActorfromClass (Utilities|Array|Get(acopy) (Variables|Default|GetCargos) (Math|Random|RandomIntegerinRange 0 4)) (Math|Transform|MakeTransform "0, 0, 0") "Undefined" 0 0))
    (bind _output_get (Variables|Default|SetSpawnedCargo _returnvalue))
    (bind _bbox (Default|GetBoundBox _output_get))
    (Transformation|SetWorldLocationAndRotation (Variables|/Game/ManipulatorRobot/Blueprints/ManipulatorRobot/BP_ManipulatorCargo.BP_ManipulatorCargo_C|GetStaticMeshCargo (Variables|Default|GetSpawnedCargo)) (+ (Math|Vector|MakeVector 0.0 0.0 (.Z (Math|Vector|BreakVector _bbox))) (+ (Math|Vector|RotateVector (Math|Vector|MakeVector (Math|Random|RandomFloatinRange (* (Variables|/Game/ManipulatorRobot/Blueprints/ManipulatorRobot/ManipulatorRobot_BP.ManipulatorRobot_BP_C|GetSkipRadius _manipulatorrobot_3) 1.5) (Variables|/Game/ManipulatorRobot/Blueprints/ManipulatorRobot/ManipulatorRobot_BP.ManipulatorRobot_BP_C|GetWorkRadius _manipulatorrobot_3)) 0.0 0.0) (Math|Rotator|MakeRotator 0.0 0.0 (Math|Random|RandomFloatinRange -1.8e+02 1.8e+02))) (Transformation|GetActorLocation _manipulatorrobot_3) (Math|Vector|MakeVector 0.0 0.0 (Math|Random|RandomFloatinRange 0.0 (/ (Variables|/Game/ManipulatorRobot/Blueprints/ManipulatorRobot/ManipulatorRobot_BP.ManipulatorRobot_BP_C|GetSeg1_len _manipulatorrobot_3) 1.0))))) (Math|Rotator|MakeRotator 0.0 0.0 (Math|Random|RandomFloatinRange -1.8e+02 1.8e+02)) false false)
    ;[1 1 1] Spawn Target at random location around the robot. Send ref of spawned Target to Cargo. Update Target bounds
    (bind _returnvalue_2 (Game|SpawnActorfromClass "/Game/ManipulatorRobot/Blueprints/ManipulatorRobot/BP_ManipulatorTarget.BP_ManipulatorTarget_C" (Math|Transform|MakeTransform (+ (Math|Vector|MakeVector 0.0 0.0 (.Z (Math|Vector|BreakVector _bbox))) (+ (Math|Vector|RotateVector (Math|Vector|MakeVector (Math|Random|RandomFloatinRange (* (Variables|/Game/ManipulatorRobot/Blueprints/ManipulatorRobot/ManipulatorRobot_BP.ManipulatorRobot_BP_C|GetSkipRadius _manipulatorrobot) 1.5) (Variables|/Game/ManipulatorRobot/Blueprints/ManipulatorRobot/ManipulatorRobot_BP.ManipulatorRobot_BP_C|GetWorkRadius _manipulatorrobot)) 0.0 0.0) (Math|Rotator|MakeRotator 0.0 0.0 (Math|Random|RandomFloatinRange -1.8e+02 1.8e+02))) (Transformation|GetActorLocation _manipulatorrobot) (Math|Vector|MakeVector 0.0 0.0 (Math|Random|RandomFloatinRange 0.0 (/ (Variables|/Game/ManipulatorRobot/Blueprints/ManipulatorRobot/ManipulatorRobot_BP.ManipulatorRobot_BP_C|GetSeg1_len _manipulatorrobot) 1.0)))))) "Undefined" 0 0))
    (Variables|/Game/ManipulatorRobot/Blueprints/ManipulatorRobot/BP_ManipulatorCargo.BP_ManipulatorCargo_C|SetTarget (Variables|Default|GetSpawnedCargo) _returnvalue_2)
    (Default|UpdateTarget (Variables|Default|GetSpawnedCargo))
    ;[1 1 1] Send Cargo to Robot
    (Default|InitCargoList _manipulatorrobot_2)
    (Default|AddCargo _manipulatorrobot_2 (Variables|Default|GetSpawnedCargo))
    (Default|Start _manipulatorrobot_2)
    (else
      (Development|PrintString "Robot is busy. Can't add Cargo" true true "(R=1.000000,G=0.922478,B=0.000000,A=1.000000)"))))

(event EventBeginPlay)

(event Collision|EventActorBeginOverlap
  (params (OtherActor :type Actor%20Object%20Reference)))

(event EventTick
  (params (DeltaSeconds :type Float%20%28single-precision%29)))

(fn ConstructionScript)