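; Player controller for the welder robot level that drives all welding robots from the keyboard.
; On BeginPlay it caches every BP_WelderRobot and checks for a BP_WeldPointSpawner to choose spawn mode.
; Space spawns a weld point through the spawner when one exists, otherwise starts every robot.
; P pauses and R resumes all cached robots.
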(event EventBeginPlay
  ;[1 1 1] Add all WelderRobot actors to the array
  (bind _outactors (Actor|GetAllActorsOfClass "/Game/WelderRobot/Blueprints/BP_WelderRobot.BP_WelderRobot_C"))
  (for _array_element _outactors
    (Utilities|Array|Add (Variables|Default|GetRobots) _array_element))
  (bind _outactors_2 (Actor|GetAllActorsOfClass "/Game/WelderRobot/Blueprints/BP_WeldPointSpawner.BP_WeldPointSpawner_C"))
  (Utilities|IsValid (Utilities|Array|Get(acopy) _outactors_2)
    (:Is%20Valid
      (Variables|Default|SetIsSpawnMode true)
      (Variables|Default|SetSpawner (Utilities|Array|Get(acopy) _outactors_2)))
    (:Is%20Not%20Valid
      (Variables|Default|SetIsSpawnMode false))))

(event Input|KeyboardEvents|SpaceBar
  (params (Key :type Key%20Structure :default "AnyKey"))
  ;[1 1 1] Starting job for all robots or start spawn welder points
  (:Pressed
    (if (Variables|Default|GetIsSpawnMode)
      (Default|SpawnWeldPoint (Variables|Default|GetSpawner))
      (else
        (for _array_element (Variables|Default|GetRobots)
          (Default|Start _array_element))))))

(event Input|KeyboardEvents|P
  (params (Key :type Key%20Structure :default "AnyKey"))
  ;[1 1 1] Activate Pause mode for all robots on the level
  (:Pressed
    (for _array_element (Variables|Default|GetRobots)
      (Default|Pause _array_element))))

(event Input|KeyboardEvents|R
  (params (Key :type Key%20Structure :default "AnyKey"))
  ;[1 1 1] Resume from pause
  (:Pressed
    (for _array_element (Variables|Default|GetRobots)
      (Default|Resume _array_element))))

(fn ConstructionScript)